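; BP_Floor is a floor segment that asks BP_FirstPersonGameMode to extend the floor when the first-person character overlaps its box.
; The construction script lays out colored arrows in two rows across the lanes and stores their transforms as spawn points.
; BeginPlay spawns random obstacle classes at shuffled points and tracks them for DestroyObstacles.
; GetAttachPoint exposes the Arrow's world transform as an attach point.
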(event OnComponentBeginOverlap(Box)
  (params (OverlappedComponent :type Primitive%20Component%20Object%20Reference) (OtherActor :type Actor%20Object%20Reference) (OtherComp :type Primitive%20Component%20Object%20Reference) (OtherBodyIndex :type Integer) (bFromSweep :type Boolean) (SweepResult :type Hit%20Result%20Structure%20%28by%20ref%29))
  (Utilities|Casting|CastToBP_FirstPersonCharacter OtherActor)
  (bind _asbp_first_person_game_mode (Utilities|Casting|CastToBP_FirstPersonGameMode (Game|GetGameMode)))
  (Default|ExtendFloor _asbp_first_person_game_mode))

(event EventBeginPlay
  (CallFunction|SpawnObstacles))

(fn ConstructionScript
  (CallFunction|SetupSpawnPoints))

(fn GetAttachPoint
  (return (Transformation|GetWorldTransform (Variables|Default|GetArrow))))

(fn SetupSpawnPoints
  (for _index (range 0 1)
    (for _array_element (Variables|---Spawn|GetLanePosition)
      (bind _returnvalue (AddComponent|AddArrowComponent false (Math|Transform|MakeTransform (Math|Vector|MakeVector (Math|Conversions|ToFloat(Integer) (+ (* _index (Variables|---Spawn|GetLane1PosX)) (Variables|---Spawn|GetLane0PosX))) _array_element 0.0))))
      (Variables|/Script/Engine.ArrowComponent|SetArrowColor _returnvalue (Utilities|Array|Get(acopy) (Variables|Default|GetArrow%20Colors) (LocalVariables|GetColorIndex)))
      (Utilities|Array|Add (Variables|Default|GetSpawnPoints) (Transformation|GetWorldTransform _returnvalue))
      (Math|Integer|IncrementInt (LocalVariables|GetColorIndex)))))

(fn SpawnObstacles
  (bind _output_get (LocalVariables|SetRandomSpawnPoints (Variables|Default|GetSpawnPoints)))
  (Utilities|Array|Shuffle _output_get)
  (for _index (range 0 (Variables|---Spawn|GetMaxObstaclesToSpawn))
    (bind _returnvalue (Game|SpawnActorfromClass (Utilities|Array|Get(acopy) (Variables|---Spawn|GetObstaclesToSpawn) (Math|Random|RandomIntegerinRange 0 (- (Utilities|Array|Length (Variables|---Spawn|GetObstaclesToSpawn)) 1))) (Utilities|Array|Get(acopy) (LocalVariables|GetRandomSpawnPoints) _index) "Undefined" "MultiplyWithRoot" 0 0))
    (Utilities|Array|Add (Variables|Default|GetSaveActors) _returnvalue)))

(fn DestroyObstacles
  (for _array_element (Variables|Default|GetSaveActors)
    (Utilities|IsValid _array_element
      (:Is%20Valid
        (Actor|DestroyActor _array_element)))))