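; Corridor floor Blueprint that scatters obstacle actors over its spawn points, overriding the parent's SpawnObstacles without calling it.
; SpawnObstacles reads SpawnInfos as a map of actor class to count and spawns each at a random SpawnPoints transform, saving it in SaveActors.
; Used indices go into PosList and duplicates are re-rolled, with no exit if every point is already taken.
; Event graph and construction script add no logic of their own.
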(event EventBeginPlay
  (|CallParentFunction) ; This node is disabled and will not be called.\nDrag off pins to build functionality.
)

(event Collision|EventActorBeginOverlap
  (params (OtherActor :type Actor%20Object%20Reference)))

(event EventTick
  (params (DeltaSeconds :type Float%20%28single-precision%29)))

(fn ConstructionScript
  (|CallParentFunction))

(fn SpawnObstacles
  (bind _spawninfos (Variables|Default|GetSpawnInfos))
  (bind _keys (Utilities|Map|Keys _spawninfos))
  (bind _values (Utilities|Map|Values _spawninfos))
  (for (_array_element _array_index) _keys
    (for _index (range 1 (Utilities|Array|Get(acopy) _values _array_index))
      (LocalVariables|SetCanSpawn true)
      (bind _output_get (LocalVariables|SetRandom (Math|Random|RandomInteger (Utilities|Array|Length (Variables|Default|GetSpawnPoints))) :!label _label))
      (if (Utilities|Array|ContainsItem (LocalVariables|GetPosList) _output_get)
        (goto _label)
        (elif (LocalVariables|GetCanSpawn)
          (Utilities|Array|Add (LocalVariables|GetPosList) _output_get)
          (bind _returnvalue (Game|SpawnActorfromClass _array_element (Utilities|Array|Get(acopy) (Variables|Default|GetSpawnPoints) _output_get) "AdjustIfPossibleButAlwaysSpawn" "MultiplyWithRoot" 0 0))
          (Utilities|Array|Add (Variables|Default|GetSaveActors) _returnvalue))))))