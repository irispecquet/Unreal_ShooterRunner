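; BP_Floor_Door is a floor variant that overrides obstacle spawning to build a row of walls with one randomly placed door, plus coins.
; The first five spawn points receive the door or a wall, and the next five each receive a coin.
; Coins are added to SaveActors for deletion if the player does not take them.
; The parent SpawnObstacles logic never runs.
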(fn ConstructionScript
  (|CallParentFunction))

(fn SpawnObstacles
  (LocalVariables|SetRandomDoorPos (Math|Random|RandomInteger 5))
  (for _index (range 0 4)
    (if (== _index (LocalVariables|GetRandomDoorPos))
      (Game|SpawnActorfromClass "/Game/Blueprints/BP_Door.BP_Door_C" (Utilities|Array|Get(acopy) (Variables|Default|GetSpawnPoints) _index) "AdjustIfPossibleButAlwaysSpawn" "MultiplyWithRoot" 0 0)
      (else
        (Game|SpawnActorfromClass "/Game/Blueprints/Obstacles/BP_Wall.BP_Wall_C" (Utilities|Array|Get(acopy) (Variables|Default|GetSpawnPoints) _index) "AdjustIfPossibleButAlwaysSpawn" "MultiplyWithRoot" 0 0))))
  (for _index_2 (range 5 9)
    (bind _returnvalue (Game|SpawnActorfromClass "/Game/Blueprints/BP_Coin.BP_Coin_C" (Utilities|Array|Get(acopy) (Variables|Default|GetSpawnPoints) _index_2) "AdjustIfPossibleButAlwaysSpawn" "MultiplyWithRoot" 0 0))
    ;[0.3646 0.3646 0.3646] Delete Coin if not taken by player
    (Utilities|Array|Add (Variables|Default|GetSaveActors) _returnvalue)))