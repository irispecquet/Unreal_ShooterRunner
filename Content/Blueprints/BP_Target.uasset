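; BP_Target is a shootable target that opens a linked door by destroying it after a set number of projectile hits.
; BP_FirstPersonProjectile hits on either the Target or SupportTarget component decrement a counter initialized from HitNeeded at BeginPlay.
; Each hit uniformly rescales ArrowTarget to the remaining-hit ratio as visual feedback.
; At zero, it destroys BPDoor and then itself, doing neither if the door reference is invalid.
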(event OnComponentHit(Target)
  (params (HitComponent :type Primitive%20Component%20Object%20Reference) (OtherActor :type Actor%20Object%20Reference) (OtherComp :type Primitive%20Component%20Object%20Reference) (NormalImpulse :type Vector :default "0, 0, 0") (Hit :type Hit%20Result%20Structure%20%28by%20ref%29))
  (Utilities|Casting|CastToBP_FirstPersonProjectile OtherActor)
  (CallFunction|ReduceScale))

(event OnComponentHit(SupportTarget)
  (params (HitComponent :type Primitive%20Component%20Object%20Reference) (OtherActor :type Actor%20Object%20Reference) (OtherComp :type Primitive%20Component%20Object%20Reference) (NormalImpulse :type Vector :default "0, 0, 0") (Hit :type Hit%20Result%20Structure%20%28by%20ref%29))
  (Utilities|Casting|CastToBP_FirstPersonProjectile OtherActor)
  (CallFunction|ReduceScale))

(event EventBeginPlay
  (Variables|---TargetInfo|SetCurrentHitNb (Math|Float|Truncate (Variables|---TargetInfo|GetHitNeeded))))

(fn ConstructionScript)

(fn ReduceScale
  (Math|Integer|DecrementInt (Variables|---TargetInfo|GetCurrentHitNb)
    (:%20%20
      (Transformation|SetWorldScale3D (Variables|Default|GetArrowTarget) (Math|Conversions|ToVector(Float) (/ (Variables|---TargetInfo|GetCurrentHitNb) (Variables|---TargetInfo|GetHitNeeded))))
      (if (<= (Variables|---TargetInfo|GetCurrentHitNb) 0)
        (CallFunction|DestroyDoor&Target)))))

(fn DestroyDoor&Target
  (bind _bp_door (Variables|Default|GetBP_Door)
    (:then
      (Actor|DestroyActor _bp_door)
      (Utilities|IsValid self
        (:Is%20Valid
          (Actor|DestroyActor))))
    (:else)))