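; BP_CoinLine is an actor that spawns a straight row of BP_Coin pickups.
; The construction script adds evenly spaced arrow components along local X, set by ArrowNumber and DistanceBetween, and stores their world transforms in SpawnPoints.
; On BeginPlay, it spawns a separate coin actor at each stored transform.
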(event EventBeginPlay
  (|CallParentFunction)
  (CallFunction|SpawnCoins))

(event Collision|EventActorBeginOverlap
  (params (OtherActor :type Actor%20Object%20Reference))
  (|CallParentFunction OtherActor) ; This node is disabled and will not be called.\nDrag off pins to build functionality.
)

(event EventTick
  (params (DeltaSeconds :type Float%20%28single-precision%29))
  (|CallParentFunction DeltaSeconds) ; This node is disabled and will not be called.\nDrag off pins to build functionality.
)

(fn ConstructionScript
  (CallFunction|SetupSpawnPoints))

(fn SetupSpawnPoints
  (for _index (range 0 (- (Variables|---Coin|GetArrowNumber) 1))
    (bind _returnvalue (AddComponent|AddArrowComponent false (Math|Transform|MakeTransform (Math|Vector|MakeVector (Math|Conversions|ToFloat(Integer) (* _index (Variables|---Coin|GetDistanceBetween))) 0.0 0.0))))
    (Utilities|Array|Add (Variables|---Coin|GetSpawnPoints) (Transformation|GetWorldTransform _returnvalue))))

(fn SpawnCoins
  (for _array_element (Variables|---Coin|GetSpawnPoints)
    (Game|SpawnActorfromClass "/Game/Blueprints/BP_Coin.BP_Coin_C" _array_element "Undefined" "MultiplyWithRoot" 0 0)))