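; BP_AIKamikaze is a suicide enemy that runs at the player and spawns BP_Explosion on arrival, then destroys itself.
; AIMoveTo drives the chase, falling back to idle and retrying after a short delay when it fails.
; Projectile hits on the capsule apply damage, updating a WBP_LifeEnemi health bar widget.
; At zero health it is destroyed without exploding.
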(event OnComponentHit(CapsuleComponent)
  (params (HitComponent :type Primitive%20Component%20Object%20Reference) (OtherActor :type Actor%20Object%20Reference) (OtherComp :type Primitive%20Component%20Object%20Reference) (NormalImpulse :type Vector :default "0, 0, 0") (Hit :type Hit%20Result%20Structure%20%28by%20ref%29))
  (Utilities|Casting|CastToBP_FirstPersonProjectile OtherActor)
  (CallFunction|Hit 25.0))

(event Custom|UpdateLifeBar
  (params (Health :type Float%20%28double-precision%29))
  ;[0.2083 0.2083 0.2083] Life
  (Variables|/Game/UserInterface/WBP_LifeEnemi.WBP_LifeEnemi_C|SetHealth (Variables|Default|GetHealth%20Bar) Health)
  (if (<= (Variables|Default|GetHealth) 0.0)
    (Actor|DestroyActor)))

(event Custom|Init%20Life
  ;[0.2083 0.2083 0.2083] Life
  (bind _aswbp_life_enemi (Utilities|Casting|CastToWBP_LifeEnemi (UserInterface|GetWidget (Variables|Default|GetHealth%20Bar%20Widget))))
  (bind _output_get (Variables|Default|SetHealth%20Bar _aswbp_life_enemi))
  (bind _output_get_2 (Variables|/Game/UserInterface/WBP_LifeEnemi.WBP_LifeEnemi_C|SetMaxHealth _output_get (Variables|Default|GetMaxHealth)))
  (bind _output_get_3 (Variables|Default|SetHealth _output_get_2))
  (CallFunction|UpdateLifeBar _output_get_3))

(event Custom|Run
  (Components|Animation|PlayAnimation (Variables|Character|GetMesh) "/Game/Characters/Mannequins/Animations/Quinn/MF_Run_Fwd.MF_Run_Fwd" true)
  (Variables|/Script/Engine.CharacterMovementComponent|SetMaxWalkSpeed (Variables|Character|GetCharacterMovement) 5e+02)
  (AI|AIMoveTo self "0, 0, 0" (Game|GetPlayerCharacter 0) 1.0 false
    (:OnSuccess
      (Game|SpawnActorfromClass "/Game/Blueprints/BP_Explosion.BP_Explosion_C" (Transformation|GetActorTransform) "Undefined" "MultiplyWithRoot" 0 0)
      (Actor|DestroyActor))
    (:OnFail
      (Components|Animation|PlayAnimation (Variables|Character|GetMesh) "/Game/Characters/Mannequins/Animations/Quinn/MF_Idle.MF_Idle" true)
      (Utilities|FlowControl|Delay 0.2)
      (CallFunction|Run))))

(event Custom|Hit
  (params (Damage :type Float%20%28double-precision%29))
  ;[0.2083 0.2083 0.2083] Life
  (Game|Damage|ApplyDamage self Damage 0 0))

(event EventBeginPlay
  (Utilities|FlowControl|Delay 1.0)
  (CallFunction|Run)
  (CallFunction|InitLife))

(event Game|Damage|EventAnyDamage
  (params (Damage :type Float%20%28single-precision%29) (DamageType :type Damage%20Type%20Object%20Reference) (InstigatedBy :type Controller%20Object%20Reference) (DamageCauser :type Actor%20Object%20Reference))
  ;[0.2083 0.2083 0.2083] Life
  (bind _output_get (Variables|Default|SetHealth (Math|Float|Clamp(Float) (- (Variables|Default|GetHealth) Damage) 0.0 (Variables|Default|GetMaxHealth))))
  (CallFunction|UpdateLifeBar _output_get))

(event EventPossessed
  (params (NewController :type Controller%20Object%20Reference))
  (Utilities|FlowControl|Delay 1.0)
  (CallFunction|Run)
  (CallFunction|InitLife))

(fn ConstructionScript)