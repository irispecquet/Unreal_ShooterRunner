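; BP_AITurret is an enemy turret that turns to face the player while they are inside its sphere trigger and has a health bar widget.
; Sphere overlaps set the range flag, which gates a smoothed yaw rotation on Tick.
; A self-calling Fire loop spawns projectiles with sound every second after a startup delay, regardless of range.
; Player projectile hits on the capsule apply damage, updating the bar and destroying the turret at zero health.
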(event OnComponentHit(CapsuleComponent)
  (params (HitComponent :type Primitive%20Component%20Object%20Reference) (OtherActor :type Actor%20Object%20Reference) (OtherComp :type Primitive%20Component%20Object%20Reference) (NormalImpulse :type Vector :default "0, 0, 0") (Hit :type Hit%20Result%20Structure%20%28by%20ref%29))
  (Utilities|Casting|CastToBP_FirstPersonProjectile OtherActor)
  (CallFunction|Hit 25.0))

(event OnComponentBeginOverlap(Sphere)
  (params (OverlappedComponent :type Primitive%20Component%20Object%20Reference) (OtherActor :type Actor%20Object%20Reference) (OtherComp :type Primitive%20Component%20Object%20Reference) (OtherBodyIndex :type Integer) (bFromSweep :type Boolean) (SweepResult :type Hit%20Result%20Structure%20%28by%20ref%29))
  ;[1 1 1] Box trigger to detect player
  (Utilities|Casting|CastToBP_FirstPersonCharacter OtherActor)
  (Variables|Default|Set_IsPlayerInRange true))

(event OnComponentEndOverlap(Sphere)
  (params (OverlappedComponent :type Primitive%20Component%20Object%20Reference) (OtherActor :type Actor%20Object%20Reference) (OtherComp :type Primitive%20Component%20Object%20Reference) (OtherBodyIndex :type Integer))
  ;[1 1 1] Box trigger to detect player
  (Utilities|Casting|CastToBP_FirstPersonCharacter OtherActor)
  (Variables|Default|Set_IsPlayerInRange false))

(event Custom|UpdateLifeBar
  (params (Health :type Float%20%28double-precision%29))
  ;[0.2083 0.2083 0.2083] Life
  (Variables|/Game/UserInterface/WBP_LifeEnemi.WBP_LifeEnemi_C|SetHealth (Variables|Default|GetHealth%20Bar) Health)
  (if (<= (Variables|Default|GetHealth) 0.0)
    (Actor|DestroyActor)))

(event Custom|Init%20Life
  ;[0.2083 0.2083 0.2083] Life
  (bind _aswbp_life_enemi (Utilities|Casting|CastToWBP_LifeEnemi (UserInterface|GetWidget (Variables|Default|GetHealth%20Bar%20Widget))))
  (bind _output_get (Variables|Default|SetHealth%20Bar _aswbp_life_enemi))
  (bind _output_get_2 (Variables|/Game/UserInterface/WBP_LifeEnemi.WBP_LifeEnemi_C|SetMaxHealth _output_get (Variables|Default|GetMaxHealth)))
  (bind _output_get_3 (Variables|Default|SetHealth _output_get_2))
  (CallFunction|UpdateLifeBar _output_get_3))

(event Custom|RotateToTarget
  ;[1 1 1] Rotate Actor
  (if (== (Variables|Default|Get_IsPlayerInRange) true)
    (Transformation|SetActorRotation (Math|Rotator|MakeRotator 0.0 0.0 (.yaw (Math|Interpolation|RInterpTo (Transformation|GetActorRotation) (Math|Rotator|FindLookatRotation (Transformation|GetActorLocation) (Transformation|GetActorLocation (Game|GetPlayerCharacter 0))) (Utilities|Time|GetWorldDeltaSeconds) 0.0))))))

(event Custom|Hit
  (params (Damage :type Float%20%28double-precision%29))
  ;[0.2083 0.2083 0.2083] Life
  (Game|Damage|ApplyDamage self Damage 0 0))

(event Custom|Fire
  (bind _returnvalue (Transformation|GetActorRotation))
  (bind _returnvalue_2 (Transformation|GetActorLocation))
  (bind _projectile_offset (Variables|Default|GetProjectile%20Offset))
  (bind _returnvalue_3 (Math|Vector|RotateVector _projectile_offset _returnvalue))
  (bind _returnvalue_4 (+ _returnvalue_2 _returnvalue_3))
  ;[0.05 0.05 0.05] Projectile Spawn Logic
  (Game|SpawnActorfromClass "/Game/Blueprints/AI/BP_AIProjectil.BP_AIProjectil_C" (Math|Transform|MakeTransform _returnvalue_4 _returnvalue) "Undefined" "OverrideRootScale" 0 0)
  (Audio|PlaySoundatLocation "/Game/Sounds/Shoot/S_ShootEnemy.S_ShootEnemy" _returnvalue_4 "0, 0, 0" 1.0 1.0 0.0 0 0 0 0) ; Play firing sound
  (Utilities|FlowControl|Delay 1.0)
  (CallFunction|Fire))

(event EventBeginPlay
  (CallFunction|InitLife)
  (Utilities|FlowControl|Delay 1.0)
  (CallFunction|Fire))

(event Game|Damage|EventAnyDamage
  (params (Damage :type Float%20%28single-precision%29) (DamageType :type Damage%20Type%20Object%20Reference) (InstigatedBy :type Controller%20Object%20Reference) (DamageCauser :type Actor%20Object%20Reference))
  ;[0.2083 0.2083 0.2083] Life
  (bind _output_get (Variables|Default|SetHealth (Math|Float|Clamp(Float) (- (Variables|Default|GetHealth) Damage) 0.0 (Variables|Default|GetMaxHealth))))
  (CallFunction|UpdateLifeBar _output_get))

(event EventTick
  (params (DeltaSeconds :type Float%20%28single-precision%29))
  (CallFunction|RotatetoTarget)
  (Utilities|FlowControl|Delay 1.0))

(fn ConstructionScript)