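; BP_Door is a door actor paired with a target that it spawns for itself.
; On BeginPlay it spawns TargetToSpawn once at the SpawnTarget transform, casts it to BP_Target and gives it a back-reference to the door.
; DestroyAnimDoor tweens the Cube downward with an ease-in, then destroys the door after a short delay.
; When the door is destroyed, it also destroys its target if still valid.
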(event Custom|DestroyAnimDoor
  (Class|TweenVectorStandardFactory|CreateTweenMoveSceneComponentby 0 (Variables|Default|GetCube) "0.000000,0.000000,-500.000000" 0.5 "EaseInExpo")
  (Utilities|FlowControl|Delay 1.0)
  (Actor|DestroyActor))

(event EventBeginPlay
  (CallFunction|InitTarget))

(event EventDestroyed
  (bind _mytarget (Variables|Default|GetMyTarget))
  (Utilities|IsValid _mytarget
    (:Is%20Valid
      (Actor|DestroyActor _mytarget))))

(fn ConstructionScript)

(fn InitTarget
  (if (not (Variables|Default|GetHasInit))
    (Variables|Default|SetHasInit true)
    (bind _returnvalue (Game|SpawnActorfromClass (Variables|Default|GetTargetToSpawn) (Transformation|GetWorldTransform (Variables|Default|GetSpawnTarget)) "Undefined" "MultiplyWithRoot" 0 0))
    (bind _asbp_target (Utilities|Casting|CastToBP_Target _returnvalue))
    (bind _output_get (Variables|Default|SetMyTarget _asbp_target))
    (Variables|/Game/Blueprints/BP_Target.BP_Target_C|SetBP_Door _output_get self)))