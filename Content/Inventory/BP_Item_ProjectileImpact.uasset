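; BP_Item_ProjectileImpact is an inventory item that upgrades the player's projectile impact as a bonus.
; Its Execute function passes the new impact and a bonus shot count to the player's UpgradeProjectileImpact, then registers itself through the player's ExecuteBonus.
; The event graph holds only disabled stubs, and construction defers to the parent class.
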(event EventBeginPlay)

(event Collision|EventActorBeginOverlap
  (params (OtherActor :type Actor%20Object%20Reference))
  (|CallParentFunction OtherActor) ; This node is disabled and will not be called.\nDrag off pins to build functionality.
)

(event EventTick
  (params (DeltaSeconds :type Float%20%28single-precision%29)))

(fn ConstructionScript
  (|CallParentFunction))

(fn Execute
  (Default|UpgradeProjectileImpact (Variables|Default|Getplayer) (Variables|Default|GetProjectileNewImpact) (Variables|Default|GetMaxShootNbWithBonus))
  (Default|ExecuteBonus (Variables|Default|Getplayer) self)
  (return 0))