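; BP_Item_Jump is an inventory item that gives the player a timed jump boost.
; Its Execute function passes the BoostJump velocity and BoostTimer duration to the player's ChangeJump, then registers itself through ExecuteBonus and returns itself.
; The event graph holds only disabled stubs and construction defers to the parent, so Execute carries all item-specific logic, along with a debug print.
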(event EventBeginPlay)

(event Collision|EventActorBeginOverlap
  (params (OtherActor :type Actor%20Object%20Reference))
  (|CallParentFunction OtherActor) ; This node is disabled and will not be called.\nDrag off pins to build functionality.
)

(event EventTick
  (params (DeltaSeconds :type Float%20%28single-precision%29)))

(fn ConstructionScript
  (|CallParentFunction))

(fn Execute
  (Development|PrintString "EXECUTE BOOST")
  (Default|ChangeJump (Variables|Default|Getplayer) (Variables|Default|GetBoostJump) (Variables|Default|GetBoostTimer))
  (Default|ExecuteBonus (Variables|Default|Getplayer) self)
  (return self))