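; Inventory boost item that changes the player's speed using a boost speed and timer.
; Execute prints a debug string, passes both boost values to the Player's ChangeSpeed, then hands itself to the Player's ExecuteBonus and returns itself.
; The construction script only calls its parent's version.
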(fn ConstructionScript
  (|CallParentFunction))

(fn Execute
  (Development|PrintString "EXECUTE BOOST")
  (Default|ChangeSpeed (Variables|Default|Getplayer) (Variables|Default|GetBoostSpeed) (Variables|Default|GetBoostTimer))
  (Default|ExecuteBonus (Variables|Default|Getplayer) self)
  (return self))