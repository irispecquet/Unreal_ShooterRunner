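; BP_Item is a pickup actor that adds itself to the first-person character's inventory on overlap.
; Overlap stores the character as Player and passes the item to AddItemToInventory.
; PickupItem plays a sound, calls DestroyComponents and returns self; the mesh and sphere are destroyed after a short delay, leaving the actor alive.
; Execute is an empty function.
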(event Custom|DestroyComponents
  (Utilities|FlowControl|Delay 0.1)
  (Components|DestroyComponent (Variables|Default|GetStaticMesh))
  (Components|DestroyComponent (Variables|Default|GetSphere)))

(event Collision|EventActorBeginOverlap
  (params (OtherActor :type Actor%20Object%20Reference))
  (bind _asbp_first_person_character (Utilities|Casting|CastToBP_FirstPersonCharacter OtherActor))
  (Variables|Default|Setplayer _asbp_first_person_character)
  (Default|AddItemtoInventory _asbp_first_person_character self))

(fn ConstructionScript)

(fn Execute
  (return 0))

(fn PickupItem
  (Audio|PlaySoundatLocation "/Game/Sounds/Bonus/PickUpBonus_Cue.PickUpBonus_Cue" (Transformation|GetActorLocation) "0, 0, 0" 1.0 1.0 0.0 0 0 0 0)
  (CallFunction|DestroyComponents)
  (return self))